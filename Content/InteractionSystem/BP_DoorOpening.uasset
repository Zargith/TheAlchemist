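; BP_DoorOpening is a door that swings open when BP_Player enters its CollisionArea and closes when the player leaves.
; Swing direction comes from the player capsule's world Y relative to the mesh, inverted when the mesh's X scale is not positive, as on mirrored doors.
; The move functions instantly set absolute world rotation to ±90 or zero degrees, with optional 2D open and close sounds.
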(event OnComponentBeginOverlap(CollisionArea)
  (params (OverlappedComponent :type Primitive%20Component%20Object%20Reference) (OtherActor :type Actor%20Object%20Reference) (OtherComp :type Primitive%20Component%20Object%20Reference) (OtherBodyIndex :type Integer) (bFromSweep :type Boolean) (SweepResult :type Hit%20Result%20Structure%20%28by%20ref%29))
  (bind _opensound (Variables|Default|GetOpenSound))
  (bind _staticmesh (Variables|Default|GetStaticMesh))
  (bind _returnvalue (Transformation|GetWorldScale _staticmesh))
  (bind _x (Math|Vector|BreakVector _returnvalue))
  (bind _returnvalue_2 (> _x 0.0))
  (bind _asbp_player (Utilities|Casting|CastToBP_Player OtherActor))
  (if (> (.Y (Math|Vector|BreakVector (Transformation|GetWorldLocation (Variables|/Script/Engine.Character|GetCapsuleComponent _asbp_player)))) (.Y (Math|Vector|BreakVector (Transformation|GetWorldLocation (Variables|Default|GetStaticMesh)))))
    (if _returnvalue_2
      (CallFunction|MovetoLeft :!label _label)
      (else
        (CallFunction|MovetoRight :!label _label_2)))
    (elif _returnvalue_2
      (goto _label_2)
      (else
        (goto _label))))
  (Utilities|IsValid _opensound
    (:Is%20Valid
      (Audio|PlaySound2D _opensound 1.0 1.0 0.0 0 0))))

(event OnComponentEndOverlap(CollisionArea)
  (params (OverlappedComponent :type Primitive%20Component%20Object%20Reference) (OtherActor :type Actor%20Object%20Reference) (OtherComp :type Primitive%20Component%20Object%20Reference) (OtherBodyIndex :type Integer))
  (bind _closesound (Variables|Default|GetCloseSound))
  (Utilities|Casting|CastToBP_Player OtherActor)
  (CallFunction|MovetoCenter)
  (Utilities|IsValid _closesound
    (:Is%20Valid
      (Audio|PlaySound2D _closesound 1.0 1.0 0.0 0 0))))

(fn ConstructionScript)

(fn MovetoLeft
  (Transformation|SetWorldRotation (Variables|Default|GetStaticMesh) "0,-90.000000, 0" false false))

(fn MovetoRight
  (Transformation|SetWorldRotation (Variables|Default|GetStaticMesh) "0,90.000000, 0" false false))

(fn MovetoCenter
  (Transformation|SetWorldRotation (Variables|Default|GetStaticMesh) "0, 0, 0" false false))
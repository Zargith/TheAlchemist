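; BP_I_Flower_var2 is a harvestable flower interactable that gives the player its item in exchange for stamina.
; On interaction it checks the player's stamina against the harvest cost read from the ItemClass defaults, then deducts that cost.
; It adds a small random amount of the item to the Inventory and destroys itself only if the add succeeds.
; Stamina is spent even when the add fails.
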(event EventBeginPlay)

(event Collision|EventActorBeginOverlap
  (params (OtherActor :type Actor%20Object%20Reference)))

(event EventTick
  (params (DeltaSeconds :type Float%20%28single-precision%29)))

(fn ConstructionScript
  (|CallParentFunction))

(fn OnInterractionAction
  (bind _itemclass (Variables|Default|GetItemClass))
  (bind _inventory (Variables|Default|Getinventory))
  (bind _iteminfos (Utilities|GetClassDefaults _itemclass))
  (bind _playerref (Variables|/Game/Systems/Inventory/Blueprints/BP_Inventory.BP_Inventory_C|GetPlayerRef _inventory))
  (bind _staminapointsusedonharvesting (Utilities|Struct|BreakS_ItemInfos _iteminfos))
  (if (>= (Variables|/Game/Blueprints/BP_Player.BP_Player_C|GetCurrentStamina _playerref) _staminapointsusedonharvesting)
    (Default|DecreaseStamina _playerref _staminapointsusedonharvesting)
    (bind _success (Default|AddItem (Variables|Default|Getinventory) (Variables|Default|GetItemClass) (Math|Random|RandomIntegerinRange 1 3)))
    (if _success
      (Actor|DestroyActor))))
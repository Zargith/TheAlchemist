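; BP_I_Mush_v5 is an interactable mushroom pickup that gives the player fly agaric items.
; On interaction it adds a random stack of one to three BP_FlyagaricItem to an inventory and destroys itself only if the add succeeds.
; A helper function prints the object's name, and the construction script just runs the parent's.
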(fn ConstructionScript
  (|CallParentFunction))

(fn OnInterractionAction
  (bind _success (Default|AddItem (Variables|Default|Getinventory) "/Game/InventorySystem/Blueprints/ItemClasses/Ingredients/Food/Mushrooms/BP_Fly-agaricItem.BP_Fly-agaricItem_C" (Math|Random|RandomIntegerinRange 1 3)))
  (if _success
    (Actor|DestroyActor)))

(fn Printname
  (Development|PrintString (Utilities|GetObjectName self)))
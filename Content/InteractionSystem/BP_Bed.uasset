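; BP_Bed is an interactable bed in the interaction system that advances the game by one day when used.
; Its interaction action calls AddDay on the Player reference.
; A separate function writes its interaction text into the prompt widget held by BP_GameInstance.
; The construction script only runs the parent's, and the event graph holds no active logic.
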(event EventBeginPlay)

(event Collision|EventActorBeginOverlap
  (params (OtherActor :type Actor%20Object%20Reference)))

(event EventTick
  (params (DeltaSeconds :type Float%20%28single-precision%29)))

(fn ConstructionScript
  (|CallParentFunction))

(fn OnInterractionAction
  (Default|AddDay (Variables|Default|Getplayer)))

(fn ChangeInteractionTxt
  (bind _asbp_game_instance (Utilities|Casting|CastToBP_GameInstance (Game|GetGameInstance)))
  (Rendering|Components|TextRender|SetText (Variables|/Game/InteractionSystem/WBP_ShowInteractKey.WBP_ShowInteractKey_C|GetInteractionTxt (Variables|/Game/Blueprints/BP_GameInstance.BP_GameInstance_C|GetInteractionWBP _asbp_game_instance)) (Variables|Default|GetInteractionText))
  (return))
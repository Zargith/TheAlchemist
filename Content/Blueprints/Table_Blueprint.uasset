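; Crafting table interactable that opens the crafting menu when the player uses it.
; On interaction it shows the CraftingMenuWidget held by the Inventory's main widget, enables the mouse cursor and switches input to Game and UI.
; Leaving its collision hides the menu, hides the cursor and restores game-only input.
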(event EventBeginPlay)

(event Collision|EventActorBeginOverlap
  (params (OtherActor :type Actor%20Object%20Reference)))

(event EventTick
  (params (DeltaSeconds :type Float%20%28single-precision%29)))

(fn ConstructionScript
  (|CallParentFunction))

(fn OnInterractionAction
  (bind _returnvalue (Game|GetPlayerController 0))
  (Widget|SetVisibility (Variables|/Game/Systems/Inventory/Widgets/MainInventoryWidget.MainInventoryWidget_C|GetCraftingMenuWidget (Variables|/Game/Systems/Inventory/Blueprints/BP_Inventory.BP_Inventory_C|GetMainWidget (Variables|Default|Getinventory))) "Visible")
  (Variables|/Script/Engine.PlayerController|SetbShowMouseCursor _returnvalue true)
  (Input|SetInputModeGameandUI _returnvalue 0 "DoNotLock" false))

(fn OnLeavingCollision
  (bind _returnvalue (Game|GetPlayerController 0))
  (Widget|SetVisibility (Variables|/Game/Systems/Inventory/Widgets/MainInventoryWidget.MainInventoryWidget_C|GetCraftingMenuWidget (Variables|/Game/Systems/Inventory/Blueprints/BP_Inventory.BP_Inventory_C|GetMainWidget (Variables|Default|Getinventory))) "Hidden")
  (Variables|/Script/Engine.PlayerController|SetbShowMouseCursor _returnvalue false)
  (Input|SetInputModeGameOnly _returnvalue))
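; Stamina potion inventory item that restores a fixed amount of the player's stamina when used.
; On use, it adds stamina and removes one unit from its inventory slot only if stamina is below maximum, then destroys its actor either way.
; The construction script caches the player as the second BP_Player found in the level, a temporary index noted for change once the extra player is removed.
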(event EventBeginPlay
  (|CallParentFunction) ; This node is disabled and will not be called.\nDrag off pins to build functionality.
)

(event Collision|EventActorBeginOverlap
  (params (OtherActor :type Actor%20Object%20Reference))
  (|CallParentFunction OtherActor) ; This node is disabled and will not be called.\nDrag off pins to build functionality.
)

(event EventTick
  (params (DeltaSeconds :type Float%20%28single-precision%29))
  (|CallParentFunction DeltaSeconds) ; This node is disabled and will not be called.\nDrag off pins to build functionality.
)

(event EventEventonUsed
  (bind _playerref (Variables|Default|GetPlayerRef))
  (if (< (Variables|/Game/Blueprints/BP_Player.BP_Player_C|GetCurrentStamina _playerref) (Variables|/Game/Blueprints/BP_Player.BP_Player_C|GetMaxStamina _playerref))
    (Default|IncreaseStamina _playerref 10)
    (Default|RemoveItematIndex (Variables|Default|GetInventory) (Variables|Default|GetIndex) 1)
    (Actor|DestroyActor)
    (else
      (Actor|DestroyActor))))

(fn ConstructionScript
  (|CallParentFunction)
  (bind _outactors (Actor|GetAllActorsOfClass "/Game/Blueprints/BP_Player.BP_Player_C"))
  (Utilities|IsValid (Utilities|Array|Get(acopy) _outactors 1)
    (:Is%20Valid
      (Variables|Default|SetPlayerRef (Utilities|Array|Get(acopy) _outactors 1)))))
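; BP_PickupActor is a world pickup that puts an item into the player's inventory on contact.
; When its Sphere component is overlapped by a BP_Player with a valid InventoryRef, it calls AddItem with its ItemToAdd class and Amount.
; On success, any leftover Rest becomes the pickup's new Amount; with nothing left over, the actor destroys itself.
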(event OnComponentBeginOverlap(Sphere)
  (params (OverlappedComponent :type Primitive%20Component%20Object%20Reference) (OtherActor :type Actor%20Object%20Reference) (OtherComp :type Primitive%20Component%20Object%20Reference) (OtherBodyIndex :type Integer) (bFromSweep :type Boolean) (SweepResult :type Hit%20Result%20Structure%20%28by%20ref%29))
  (bind _asbp_player (Utilities|Casting|CastToBP_Player OtherActor))
  (Utilities|IsValid (Variables|/Game/Blueprints/BP_Player.BP_Player_C|GetInventoryRef _asbp_player)
    (:Is%20Valid
      (bind (_success _rest_) (Default|AddItem (Variables|/Game/Blueprints/BP_Player.BP_Player_C|GetInventoryRef _asbp_player) (Variables|Default|GetItemToAdd) (Variables|Default|GetAmount)))
      (if _success
        (if (> _rest_ 0)
          (Variables|Default|SetAmount _rest_)
          (else
            (Actor|DestroyActor)))))))

(event EventBeginPlay)

(event Collision|EventActorBeginOverlap
  (params (OtherActor :type Actor%20Object%20Reference)))

(event EventTick
  (params (DeltaSeconds :type Float%20%28single-precision%29)))

(fn ConstructionScript)
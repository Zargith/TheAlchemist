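; BP_CyclesManager is an actor that holds a day counter for the game's cycle system.
; It exposes functions to increment the day, reset it to 1 and print the current count.
; The construction script sets Days to 1, then checks for 365 to reset, so that branch never triggers.
; AddDay also looks up BP_Player actors without using the result, and the event graph is inactive.
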(event EventBeginPlay)

(event Collision|EventActorBeginOverlap
  (params (OtherActor :type Actor%20Object%20Reference)))

(event EventTick
  (params (DeltaSeconds :type Float%20%28single-precision%29)))

(fn ConstructionScript
  (Variables|Default|SetDays 1)
  (if (== (Variables|Default|GetDays) 365)
    (CallFunction|ResetDays)))

(fn GetDayNb
  (Development|PrintString (Utilities|String|ToString(Integer) (Variables|Default|GetDays))))

(fn ResetDays
  (Variables|Default|SetDays 1))

(fn AddDay
  (Variables|Default|SetDays (+ (Variables|Default|GetDays) 1))
  (bind _outactors (Actor|GetAllActorsOfClass "/Game/Blueprints/BP_Player.BP_Player_C")))
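; Base quest Blueprint that tracks a quest's active and completed sub-goals, with empty completed/failed events as hooks.
; CompleteSubGoal records results, appends description updates, then chains following goals or ends the quest through QuestManager.
; AddGoalForIndex recursively auto-completes goals the inventory already satisfies (with a hard-coded Quest_Tuto_2 exception), otherwise spawning sub-goal widgets.
; It directly updates the quest widget and journal, removing its entries on end or cancel.
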(event Custom|OnGoalFailed
  (params (GoalIndex :type Integer)))

(event Custom|OnQuestCancelled
  (CallFunction|RemoveWidgets)
  (Default|CancelQuest (Variables|DoNotTouch|GetQuestManager) self))

(event Custom|OnGoalCompleted
  (params (GoalIndex :type Integer)))

(fn ConstructionScript)

(fn UpdateSubGoals
  (Utilities|Array|Clear (Variables|DoNotTouch|GetCurrentGoals))
  (for _array_element (Variables|DoNotTouch|GetCurrentGoalIndices)
    (Utilities|Array|Add (Variables|DoNotTouch|GetCurrentGoals) (Utilities|Array|Get(acopy) (.SubGoals (Utilities|Struct|Breaks_QuestInfo (Variables|QuestInformation|GetQuestInfo))) _array_element)))
  (return))

(fn SetupStartingGoals
  (Utilities|Array|Clear (Variables|DoNotTouch|GetCurrentGoalIndices))
  (Variables|DoNotTouch|SetCurrentDescription (.Description (Utilities|Struct|Breaks_QuestInfo (Variables|QuestInformation|GetQuestInfo))))
  (for _array_element (Variables|QuestInformation|GetStartingSubGoalIndices)
    (CallFunction|AddGoalforIndex _array_element))
  (Utilities|Array|Resize (Variables|DoNotTouch|GetCurrentAmount) (Utilities|Array|Length (Variables|DoNotTouch|GetCurrentGoalIndices)))
  (CallFunction|UpdateSubGoals)
  (return))

(fn GotoNextSubGoal
  (bind _currentgoalindices (Variables|DoNotTouch|GetCurrentGoalIndices))
  (bind _currentgoalindices_2 (Variables|DoNotTouch|GetCurrentGoalIndices))
  (bind _maxvalue (Math|Integer|MaxOfIntArray _currentgoalindices))
  (bind _returnvalue (+ _maxvalue 1))
  (if (<= _returnvalue (Utilities|Array|LastIndex (.SubGoals (Utilities|Struct|Breaks_QuestInfo (Variables|QuestInformation|GetQuestInfo)))))
    (bind _output_get (LocalVariables|SetNextIndex _returnvalue))
    (Utilities|Array|Clear _currentgoalindices_2)
    (Utilities|Array|Add _currentgoalindices_2 _output_get)
    (CallFunction|UpdateSubGoals)
    (return true)
    (else
      (return false))))

(fn CompleteSubGoal
  (params (SubGoalIndex :type Integer) (Fail? :type Boolean))
  (bind _currentgoalindices (Variables|DoNotTouch|GetCurrentGoalIndices))
  (bind _questwidget (Variables|DoNotTouch|GetQuestWidget))
  (bind _questwidget_2 (Variables|DoNotTouch|GetQuestWidget))
  (bind _subgoalwidget (Variables|/Game/Systems/Quest/Widget/WBP_Quest.WBP_Quest_C|GetSubGoalWidget _questwidget))
  (LocalVariables|SetlocalFail? Fail?)
  (LocalVariables|SetlocalGoalIndex SubGoalIndex)
  (if (Utilities|Array|ContainsItem (Variables|DoNotTouch|GetCurrentGoalIndices) (LocalVariables|GetlocalGoalIndex))
    (bind _output_get (LocalVariables|SetlocalCompletedGoal (Utilities|Array|Get(acopy) (.SubGoals (Utilities|Struct|Breaks_QuestInfo (Variables|QuestInformation|GetQuestInfo))) (LocalVariables|GetlocalGoalIndex))))
    (Utilities|Array|Add (Variables|DoNotTouch|GetCompletedSubGoals) (Utilities|Struct|Makes_CompletedGoal (LocalVariables|GetlocalGoalIndex) _output_get (not (LocalVariables|GetlocalFail?))))
    (if (and (.UpdateQuestDescription? (Utilities|Struct|Breaks_GoalInfo (LocalVariables|GetlocalCompletedGoal))) (not (LocalVariables|GetlocalFail?)))
      (Variables|DoNotTouch|SetCurrentDescription (Utilities|Text|FormatText "{Current}{Next}" (Variables|DoNotTouch|GetCurrentDescription) (.UpdatedDescription (Utilities|Struct|Breaks_GoalInfo (LocalVariables|GetlocalCompletedGoal)))))
      (if (CallFunction|SelectedinJournal?)
        (Default|UpdateDescription (Variables|/Game/Systems/MainWidget.MainWidget_C|GetQuestJournal (Variables|/Game/Systems/Quest/BluePrints/BP_QuestManager.BP_QuestManager_C|GetMainWidget (Variables|DoNotTouch|GetQuestManager))))))
    (Utilities|Array|RemoveItem (Variables|DoNotTouch|GetCurrentGoals) (LocalVariables|GetlocalCompletedGoal))
    (LocalVariables|SetlocalWidgetIndex (Utilities|Array|FindItem _currentgoalindices (LocalVariables|GetlocalGoalIndex)))
    (Utilities|Array|RemoveIndex (Variables|DoNotTouch|GetCurrentAmount) (Utilities|Array|FindItem _currentgoalindices (LocalVariables|GetlocalGoalIndex)))
    (Utilities|Array|RemoveItem _currentgoalindices (LocalVariables|GetlocalGoalIndex))
    (Widget|RemovefromParent (Utilities|Array|Get(acopy) _subgoalwidget (LocalVariables|GetlocalWidgetIndex)))
    (Utilities|Array|RemoveIndex _subgoalwidget (LocalVariables|GetlocalWidgetIndex))
    (if (LocalVariables|GetlocalFail?)
      (CallFunction|OnGoalFailed (LocalVariables|GetlocalGoalIndex))
      (if (.FailMeansQuestFail? (Utilities|Struct|Breaks_GoalInfo (LocalVariables|GetlocalCompletedGoal)))
        _
        (else
          (if (CallFunction|SelectedinJournal?) :!label _label
            (Default|GenerateSubGoals (Variables|/Game/Systems/MainWidget.MainWidget_C|GetQuestJournal (Variables|/Game/Systems/Quest/BluePrints/BP_QuestManager.BP_QuestManager_C|GetMainWidget (Variables|DoNotTouch|GetQuestManager)))))
          (if (and (== (LocalVariables|GetlocalGoalIndex) (Variables|DoNotTouch|GetSelectedSubGoalIndex)) (== (Variables|/Game/Systems/Quest/BluePrints/BP_QuestManager.BP_QuestManager_C|GetCurrentQuest (Variables|DoNotTouch|GetQuestManager)) self))
            (Default|SelectSubGoal _questwidget_2 (Utilities|Array|Get(acopy) (Variables|/Game/Systems/Quest/Widget/WBP_Quest.WBP_Quest_C|GetSubGoalWidget _questwidget_2))))
          (return true)))
      (else
        (CallFunction|OnGoalCompleted (LocalVariables|GetlocalGoalIndex))
        (if (.CompletesQuest? (Utilities|Struct|Breaks_GoalInfo (LocalVariables|GetlocalCompletedGoal)))
          _
          (else
            (for _array_element (.FollowingSubGoalIndices (Utilities|Struct|Breaks_GoalInfo (LocalVariables|GetlocalCompletedGoal)))
              (CallFunction|AddGoalforIndex _array_element))
            (goto _label)))))
    (for _array_element_2 (Variables|DoNotTouch|GetCurrentGoalIndices)
      (Utilities|Array|Add (Variables|DoNotTouch|GetCompletedSubGoals) (Utilities|Struct|Makes_CompletedGoal _array_element_2 (CallFunction|GoalatIndex _array_element_2) false)))
    (Utilities|Array|Clear (Variables|DoNotTouch|GetCurrentGoalIndices))
    (Utilities|Array|Clear (Variables|DoNotTouch|GetCurrentAmount))
    (Utilities|Array|Clear (Variables|DoNotTouch|GetCurrentGoals))
    (Variables|DoNotTouch|SetCurrentState (select (LocalVariables|GetlocalFail?) "NewEnumerator2" "NewEnumerator1"))
    (CallFunction|RemoveWidgets)
    (Default|EndQuest (Variables|DoNotTouch|GetQuestManager) self)
    (return true)
    (else
      (return false))))

(fn GoalatIndex
  (params (Index :type Integer))
  (return (Utilities|Array|Get(acopy) (.SubGoals (Utilities|Struct|Breaks_QuestInfo (Variables|QuestInformation|GetQuestInfo))) Index)))

(fn SelectedinJournal?
  (bind _questmanager (Variables|DoNotTouch|GetQuestManager))
  (bind _mainwidget (Variables|/Game/Systems/Quest/BluePrints/BP_QuestManager.BP_QuestManager_C|GetMainWidget _questmanager))
  (bind _questjournal (Variables|/Game/Systems/MainWidget.MainWidget_C|GetQuestJournal _mainwidget))
  (bind _selectedquest (Variables|/Game/Systems/Quest/Widget/QuestJournal.QuestJournal_C|GetSelectedQuest _questjournal))
  (return (and (Utilities|IsValid _selectedquest) (== _selectedquest self))))

(fn GoalAlreadyFound?
  (params (GoalIndex :type Integer))
  (bind _goal (CallFunction|GoalatIndex GoalIndex))
  (bind (_type _customgoal_ _goaltext _additionalname _amount _location _updatequestdescription_ _updateddescription _followingsubgoalindices _goalclass) (Utilities|Struct|Breaks_GoalInfo _goal))
  (if (and (== (Utilities|GetClass (Variables|/Game/Systems/Quest/BluePrints/BP_QuestManager.BP_QuestManager_C|GetCurrentQuest (Variables|DoNotTouch|GetQuestManager))) "/Game/Systems/Quest/BluePrints/Quests/Tuto/Quest_Tuto_2.Quest_Tuto_2_C") (or (== GoalIndex 1) (== GoalIndex 2)))
    _
    (elif (or (Utilities|Enum|Equal(Enum) _type "NewEnumerator2") (Utilities|Enum|Equal(Enum) _type "NewEnumerator1"))
      _
      (else
        (return false))))
  (bind _totalamount (Default|GetTotalAmountOfItem (Variables|/Game/Blueprints/BP_Player.BP_Player_C|GetInventoryRef (Variables|/Game/Systems/Quest/BluePrints/BP_QuestManager.BP_QuestManager_C|GetPlayer (Variables|DoNotTouch|GetQuestManager))) _goalclass))
  (return (>= _totalamount _amount)))

(fn AddGoalforIndex
  (params (I :type Integer))
  (bind _questwidget (Variables|DoNotTouch|GetQuestWidget))
  (bind _output_get (LocalVariables|SetlocalIndex I))
  (if (CallFunction|GoalAlreadyFound? _output_get)
    (Utilities|Array|Add (Variables|DoNotTouch|GetCompletedSubGoals) (Utilities|Struct|Makes_CompletedGoal (LocalVariables|GetlocalIndex) (CallFunction|GoalatIndex (LocalVariables|GetlocalIndex)) true))
    (CallFunction|OnGoalCompleted (LocalVariables|GetlocalIndex))
    (if (.UpdateQuestDescription? (Utilities|Struct|Breaks_GoalInfo (CallFunction|GoalatIndex (LocalVariables|GetlocalIndex))))
      (Variables|DoNotTouch|SetCurrentDescription (Utilities|Text|FormatText "{Current}{Next}" (Variables|DoNotTouch|GetCurrentDescription) (.UpdatedDescription (Utilities|Struct|Breaks_GoalInfo (CallFunction|GoalatIndex (LocalVariables|GetlocalIndex))))))
      (if (CallFunction|SelectedinJournal?)
        (Default|UpdateDescription (Variables|/Game/Systems/MainWidget.MainWidget_C|GetQuestJournal (Variables|/Game/Systems/Quest/BluePrints/BP_QuestManager.BP_QuestManager_C|GetMainWidget (Variables|DoNotTouch|GetQuestManager))))))
    (for _array_element (.FollowingSubGoalIndices (Utilities|Struct|Breaks_GoalInfo (CallFunction|GoalatIndex (LocalVariables|GetlocalIndex))))
      (CallFunction|AddGoalforIndex _array_element))
    (return)
    (else
      (bind _returnvalue (Utilities|Array|Add (Variables|DoNotTouch|GetCurrentGoalIndices) (LocalVariables|GetlocalIndex)))
      (if (> _returnvalue (Utilities|Array|LastIndex (Variables|DoNotTouch|GetCurrentAmount)))
        (Utilities|Array|Add (Variables|DoNotTouch|GetCurrentAmount) 0))
      (Utilities|Array|Add (Variables|DoNotTouch|GetCurrentGoals) (CallFunction|GoalatIndex (LocalVariables|GetlocalIndex)))
      (bind _returnvalue_2 (UserInterface|CreateWidget "/Game/Systems/Quest/Widget/WBP_SubGoal.WBP_SubGoal_C" 0 (CallFunction|GoalatIndex (LocalVariables|GetlocalIndex)) self (Variables|DoNotTouch|GetQuestWidget)))
      (Utilities|Array|Add (Variables|/Game/Systems/Quest/Widget/WBP_Quest.WBP_Quest_C|GetSubGoalWidget _questwidget) _returnvalue_2)
      (Widget|Panel|AddChild (Variables|/Game/Systems/Quest/Widget/WBP_Quest.WBP_Quest_C|GetSubGoalBox _questwidget) _returnvalue_2)
      (return))))

(fn RemoveWidgets
  (bind _questmanager (Variables|DoNotTouch|GetQuestManager))
  (bind _listentrywidget (Variables|DoNotTouch|GetListEntryWidget))
  (bind _mainwidget (Variables|/Game/Systems/Quest/BluePrints/BP_QuestManager.BP_QuestManager_C|GetMainWidget _questmanager))
  (Utilities|Array|RemoveItem (Variables|/Game/Systems/MainWidget.MainWidget_C|GetQuestWidget _mainwidget) (Variables|DoNotTouch|GetQuestWidget))
  (Utilities|Array|RemoveItem (Variables|/Game/Systems/Quest/Widget/QuestJournal.QuestJournal_C|GetAllQuestEntries (Variables|/Game/Systems/MainWidget.MainWidget_C|GetQuestJournal _mainwidget)) _listentrywidget)
  (Widget|RemovefromParent _listentrywidget)
  (return))

(fn CreateClassfromGoalInfo
  (params (SubGoal :type S%20Goal%20Info%20Structure))
  (return))
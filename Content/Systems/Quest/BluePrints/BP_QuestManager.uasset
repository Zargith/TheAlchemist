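; Quest manager that adds, selects, cancels and ends quests, keeping the quest list and journal in sync with their state.
; Each unique quest class spawns a quest actor; ending one files it by state, pays gold on completion and selects the next.
; Switching sub-quests spawns a goal actor at its location.
; Player movement updates a map arrow toward it, toggled by horizontal distance through paired DoOnce gates.
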(event Custom|OnSwitchSubQuest
  (bind _currentquest (Variables|Default|GetCurrentQuest))
  (Utilities|IsValid (Variables|Default|GetCurrentGoalActor)
    (:Is%20Valid
      (Actor|DestroyActor (Variables|Default|GetCurrentGoalActor)))
    (:Is%20Not%20Valid
      _))
  (bind _output_get (Variables|Default|SetCurrentSubGoal (Utilities|Array|Get(acopy) (.SubGoals (Utilities|Struct|Breaks_QuestInfo (Variables|/Game/Systems/Quest/BluePrints/BP_MasterQuest.BP_MasterQuest_C|GetQuestInfo _currentquest))) (Variables|/Game/Systems/Quest/BluePrints/BP_MasterQuest.BP_MasterQuest_C|GetSelectedSubGoalIndex _currentquest))))
  (if (.hasLocation? (Utilities|Struct|Breaks_GoalLocation (.Location (Utilities|Struct|Breaks_GoalInfo _output_get))))
    (bind _returnvalue (Game|SpawnActorfromClass "/Game/Systems/Quest/BluePrints/BP_GoalActor.BP_GoalActor_C" (Math|Transform|MakeTransform (.Location (Utilities|Struct|Breaks_GoalLocation (.Location (Utilities|Struct|Breaks_GoalInfo _output_get)))) "0, 0, 0" "1,1,1") "AlwaysSpawn" 0 (.UseRadius? (Utilities|Struct|Breaks_GoalInfo _output_get)) (.Radius (Utilities|Struct|Breaks_GoalInfo _output_get)) (.CircleColor (Utilities|Struct|Breaks_GoalInfo _output_get)) 0))
    (Variables|Default|SetCurrentGoalActor _returnvalue)
    (Variables|Default|SetCurrentDistance (CallFunction|DistancetoGoal))
    (CallFunction|UpdateDirectionArrow)
    (Widget|SetVisibility (Variables|/Game/Systems/Quest/Widget/MiniMap.MiniMap_C|GetDirectionArrow (Variables|/Game/Systems/MainWidget.MainWidget_C|GetMap (Variables|Default|GetMainWidget))) (select (> (Variables|Default|GetCurrentDistance) (Variables|Default|GetShowDirectionArrowAmount)) "HitTestInvisible" "Hidden"))
    (else
      (Variables|Default|SetCurrentGoalActor 0)
      (Widget|SetVisibility (Variables|/Game/Systems/Quest/Widget/MiniMap.MiniMap_C|GetDirectionArrow (Variables|/Game/Systems/MainWidget.MainWidget_C|GetMap (Variables|Default|GetMainWidget))) "Hidden"))))

(event Custom|OnPlayerMove
  (Utilities|IsValid (Variables|Default|GetCurrentGoalActor)
    (:Is%20Valid
      (bind _output_get (Variables|Default|SetCurrentDistance (CallFunction|DistancetoGoal)))
      (Math|Integer|CompareInt _output_get (Variables|Default|GetShowDirectionArrowAmount)
        (:>
          _)
        (:==
          _)
        (:<
          (Utilities|FlowControl|DoOnce false :!label _label
            (:Completed
              (Widget|SetVisibility (Variables|/Game/Systems/Quest/Widget/MiniMap.MiniMap_C|GetDirectionArrow (Variables|/Game/Systems/MainWidget.MainWidget_C|GetMap (Variables|Default|GetMainWidget))) "Hidden")
              (goto _label_2 Reset)))))
      (CallFunction|UpdateDirectionArrow)
      (Utilities|FlowControl|DoOnce false :!label _label_2
        (:Completed
          (Widget|SetVisibility (Variables|/Game/Systems/Quest/Widget/MiniMap.MiniMap_C|GetDirectionArrow (Variables|/Game/Systems/MainWidget.MainWidget_C|GetMap (Variables|Default|GetMainWidget))) "HitTestInvisible")
          (goto _label Reset))))))

(fn ConstructionScript)

(fn SelectNewQuest
  (params (Quest :type BP%20Master%20Quest%20Object%20Reference) (SubGoal :type WBP%20Sub%20Goal%20Object%20Reference) (Loaded? :type Boolean))
  (Utilities|IsValid (Variables|Default|GetCurrentQuest)
    (:Is%20Valid
      (Widget|SetIsEnabled (Variables|/Game/Systems/Quest/Widget/WBP_Quest.WBP_Quest_C|GetQuestName (Variables|/Game/Systems/Quest/BluePrints/BP_MasterQuest.BP_MasterQuest_C|GetQuestWidget (Variables|Default|GetCurrentQuest))) false)
      (Default|SelectSubGoal (Variables|/Game/Systems/Quest/BluePrints/BP_MasterQuest.BP_MasterQuest_C|GetQuestWidget (Variables|Default|GetCurrentQuest))))
    (:Is%20Not%20Valid
      _))
  (bind _output_get (Variables|Default|SetCurrentQuest Quest))
  (Default|OnQuestSelected (Variables|/Game/Systems/Quest/BluePrints/BP_MasterQuest.BP_MasterQuest_C|GetQuestWidget _output_get) SubGoal)
  (return))

(fn AddNewQuest
  (params (QuestClass :type BP%20Master%20Quest%20Class%20Reference) (DirectlyStart? :type Boolean))
  (bind _mainwidget (Variables|Default|GetMainWidget))
  (LocalVariables|SetLocalClass QuestClass)
  (LocalVariables|Setstart? DirectlyStart?)
  (if (and (Utilities|IsValidClass QuestClass) (not (Utilities|Array|ContainsItem (Variables|Default|GetAllQuestClasses) QuestClass)))
    (Utilities|Array|Add (Variables|Default|GetAllQuestClasses) (LocalVariables|GetLocalClass))
    (bind _returnvalue (Game|SpawnActorfromClass (LocalVariables|GetLocalClass) (Math|Transform|MakeTransform "0, 0, 0" "0, 0, 0" "1,1,1") "AlwaysSpawn" 0 self 0))
    (bind _output_get (LocalVariables|SetLocalQuestActor _returnvalue))
    (Utilities|Array|Add (Variables|Default|GetCurrentQuestActors) _output_get)
    (bind _widget (Default|AddQuesttoList (Variables|Default|GetMainWidget) _output_get))
    (bind _output_get_2 (Variables|/Game/Systems/Quest/BluePrints/BP_MasterQuest.BP_MasterQuest_C|SetQuestWidget (LocalVariables|GetLocalQuestActor) _widget))
    (Default|SetupStartingGoals (LocalVariables|GetLocalQuestActor))
    (Default|UpdateQuest _output_get_2)
    (Default|AddEntry (Variables|/Game/Systems/MainWidget.MainWidget_C|GetQuestJournal (Variables|Default|GetMainWidget)) (LocalVariables|GetLocalQuestActor))
    (if (or (LocalVariables|Getstart?) (<= (Utilities|Array|Length (Variables|Default|GetCurrentQuestActors)) 1))
      (CallFunction|SelectNewQuest (LocalVariables|GetLocalQuestActor) (Utilities|Array|Get(acopy) (Variables|/Game/Systems/Quest/Widget/WBP_Quest.WBP_Quest_C|GetSubGoalWidget (Variables|/Game/Systems/Quest/BluePrints/BP_MasterQuest.BP_MasterQuest_C|GetQuestWidget (LocalVariables|GetLocalQuestActor)))) false))
    (if (Variables|/Game/Systems/MainWidget.MainWidget_C|GetSlideOut? _mainwidget)
      (UserInterface|Animation|PlayAnimation _mainwidget (Variables|/Game/Systems/MainWidget.MainWidget_C|GetSlideOut _mainwidget) 0.0 1 "Reverse" 1.0 false)
      (Variables|/Game/Systems/MainWidget.MainWidget_C|SetSlideOut? _mainwidget false))
    (return true)
    (else
      (return false))))

(fn DistancetoGoal
  (bind _player (Variables|Default|GetPlayer))
  (bind _currentgoalactor (Variables|Default|GetCurrentGoalActor))
  (bind _returnvalue (Transformation|GetActorLocation _currentgoalactor))
  (bind _returnvalue_2 (Transformation|GetActorLocation _player))
  (return (Math|Float|Round (/ (Math|Vector|VectorLength (- (Math|Vector|MakeVector (.x _returnvalue_2) (.y _returnvalue_2) 0.0) (Math|Vector|MakeVector (.x _returnvalue) (.y _returnvalue) 0.0))) 1e+02))))

(fn UpdateDirectionArrow
  (Class|Widget|SetRenderTransformAngle (Variables|/Game/Systems/Quest/Widget/MiniMap.MiniMap_C|GetDirectionArrow (Variables|/Game/Systems/MainWidget.MainWidget_C|GetMap (Variables|Default|GetMainWidget))) (.Yaw (Math|Rotator|BreakRotator (Math|Rotator|FindLookatRotation (Transformation|GetActorLocation (Variables|Default|GetPlayer)) (Transformation|GetActorLocation (Variables|Default|GetCurrentGoalActor))))))
  (return))

(fn HasCurrentQuest?
  (params (QuestClass :type BP%20Master%20Quest%20Class%20Reference))
  (bind _array_element (Utilities|Array|ForEachLoopwithBreak (Variables|Default|GetCurrentQuestActors) :!label _label)
    (:LoopBody
      (if (== (Utilities|GetClass _array_element) QuestClass)
        (LocalVariables|SetfoundQuest _array_element)
        (goto _label Break)))
    (:Completed
      (Utilities|IsValid (LocalVariables|GetfoundQuest)
        (:Is%20Valid
          (return true (LocalVariables|GetfoundQuest)))
        (:Is%20Not%20Valid
          (return false 0))))))

(fn EndQuest
  (params (Quest :type BP%20Master%20Quest%20Object%20Reference))
  (bind _currentgoalactor (Variables|Default|GetCurrentGoalActor))
  (bind _currentquestactors (Variables|Default|GetCurrentQuestActors))
  (bind _output (Utilities|Array|Get(acopy) _currentquestactors))
  (bind _output_get (LocalVariables|SetlocalQuest Quest))
  (Utilities|Array|RemoveItem (Variables|Default|GetCurrentQuestActors) _output_get)
  (Utilities|Array|Add (Utilities|Select :Index (Variables|/Game/Systems/Quest/BluePrints/BP_MasterQuest.BP_MasterQuest_C|GetCurrentState (LocalVariables|GetlocalQuest)) :NewEnumerator0 (Variables|Default|GetCurrentQuestActors) :NewEnumerator1 (Variables|Default|GetCompletedQuest) :NewEnumerator2 (Variables|Default|GetFailedQuestActors)) (LocalVariables|GetlocalQuest))
  (Default|AddEntry (Variables|/Game/Systems/MainWidget.MainWidget_C|GetQuestJournal (Variables|Default|GetMainWidget)) (LocalVariables|GetlocalQuest))
  (if (== (LocalVariables|GetlocalQuest) (Variables|Default|GetCurrentQuest))
    (Variables|Default|SetCurrentQuest 0)
    (Utilities|IsValid _currentgoalactor
      (:Is%20Valid
        (Actor|DestroyActor _currentgoalactor)
        (Widget|SetVisibility (Variables|/Game/Systems/Quest/Widget/MiniMap.MiniMap_C|GetDirectionArrow (Variables|/Game/Systems/MainWidget.MainWidget_C|GetMap (Variables|Default|GetMainWidget))) "Hidden"))
      (:Is%20Not%20Valid
        _))
    (Utilities|IsValid _output
      (:Is%20Valid
        (CallFunction|SelectNewQuest _output (Utilities|Array|Get(acopy) (Variables|/Game/Systems/Quest/Widget/WBP_Quest.WBP_Quest_C|GetSubGoalWidget (Variables|/Game/Systems/Quest/BluePrints/BP_MasterQuest.BP_MasterQuest_C|GetQuestWidget _output))) false))
      (:Is%20Not%20Valid
        _)))
  (if (Default|SelectedinJournal? (LocalVariables|GetlocalQuest))
    (Default|OnQuestClicked (Variables|/Game/Systems/MainWidget.MainWidget_C|GetQuestJournal (Variables|Default|GetMainWidget))))
  (if (Utilities|Enum|Equal(Enum) (Variables|/Game/Systems/Quest/BluePrints/BP_MasterQuest.BP_MasterQuest_C|GetCurrentState (LocalVariables|GetlocalQuest)) "NewEnumerator1")
    (Default|IncreaseGold (Variables|Default|GetPlayer) (Utilities|Struct|Breaks_QuestReward (.CompletionReward (Utilities|Struct|Breaks_QuestInfo (Variables|/Game/Systems/Quest/BluePrints/BP_MasterQuest.BP_MasterQuest_C|GetQuestInfo (LocalVariables|GetlocalQuest))))))
    (return)
    (else
      (return))))

(fn CompleteGoals)

(fn CancelQuest
  (params (QuestActor :type BP%20Master%20Quest%20Object%20Reference))
  (bind _currentgoalactor (Variables|Default|GetCurrentGoalActor))
  (bind _currentquestactors (Variables|Default|GetCurrentQuestActors))
  (bind _output (Utilities|Array|Get(acopy) _currentquestactors))
  (bind _output_get (LocalVariables|SetLocalQuest QuestActor))
  (Utilities|Array|RemoveItem (Variables|Default|GetCurrentQuestActors) _output_get)
  (if (== (LocalVariables|GetLocalQuest) (Variables|Default|GetCurrentQuest))
    (Variables|Default|SetCurrentQuest 0)
    (Utilities|IsValid _currentgoalactor
      (:Is%20Valid
        (Actor|DestroyActor _currentgoalactor)
        (Widget|SetVisibility (Variables|/Game/Systems/Quest/Widget/MiniMap.MiniMap_C|GetDirectionArrow (Variables|/Game/Systems/MainWidget.MainWidget_C|GetMap (Variables|Default|GetMainWidget))) "Hidden"))
      (:Is%20Not%20Valid
        _))
    (Utilities|IsValid _output
      (:Is%20Valid
        (CallFunction|SelectNewQuest _output (Utilities|Array|Get(acopy) (Variables|/Game/Systems/Quest/Widget/WBP_Quest.WBP_Quest_C|GetSubGoalWidget (Variables|/Game/Systems/Quest/BluePrints/BP_MasterQuest.BP_MasterQuest_C|GetQuestWidget _output))) false))
      (:Is%20Not%20Valid
        _)))
  (if (not (Default|SelectedinJournal? (LocalVariables|GetLocalQuest)))
    (if false
      _)))
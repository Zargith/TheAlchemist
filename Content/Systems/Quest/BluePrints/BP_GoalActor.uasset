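; BP_GoalActor is a quest goal marker that represents a location on the minimap as either an icon or a radius circle.
; The construction script uses UseRadius to pick which sprite shows, scales the circle from Radius and tints it with CircleColor.
; On BeginPlay it makes the player character its owner and sets Owner No See on the icon, hiding it from that player's own view.
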(event EventBeginPlay
  (Actor|SetOwner (Game|GetPlayerCharacter 0))
  (Class|PrimitiveComponent|SetOwnerNoSee (Variables|Default|GetMiniMapIcon) true))

(fn ConstructionScript
  (bind _radius (Variables|Default|GetRadius))
  (bind _minimapr (Variables|Default|GetMiniMapR))
  (bind _returnvalue (/ _radius 5e+02))
  (Rendering|SetVisibility (Variables|Default|GetMiniMapIcon) (not (Variables|Default|GetUseRadius?)) false)
  (Transformation|SetRelativeScale3D _minimapr (Math|Vector|MakeVector _returnvalue 1.0 _returnvalue))
  (Rendering|SetVisibility _minimapr (Variables|Default|GetUseRadius?) false)
  (Sprite|SetSpriteColor _minimapr (Variables|Default|GetCircleColor)))
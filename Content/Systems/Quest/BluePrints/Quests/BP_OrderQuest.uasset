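; Randomly generated order quest asking for either a quantity of an ingredient to collect or a potion to make and deliver.
; On BeginPlay it picks the order type, item class and amount, then fills QuestInfo and its sub-goal with formatted text.
; Rewards scale from item value times quantity, with a higher markup for potions.
; CreateClassFromGoalInfo rebuilds QuestInfo from a given sub-goal, always using the potion-style description.
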(event EventBeginPlay
  (bind _allpotionitemclass (Variables|Default|GetAllPotionItemClass))
  (bind _allingredientitemclass (Variables|Default|GetAllIngredientItemClass))
  (if (Math|Random|RandomBool)
    (bind _output_get (Variables|Default|SetIngredient (Utilities|Array|Get(acopy) _allingredientitemclass (Math|Random|RandomInteger (Utilities|Array|Length _allingredientitemclass)))))
    (bind _output_get_2 (Variables|Default|SetDesiredIngredients (Math|Random|RandomIntegerinRange 4 10)))
    (bind _structout (Utilities|Struct|Setmembersins_GoalInfo (Utilities|Array|Get(acopy) (.SubGoals (Utilities|Struct|Breaks_QuestInfo (Variables|Default|GetQuestInfo)))) "NewEnumerator1" true (Utilities|Text|FormatText "Collect {quantity}x {name}" _output_get_2 (.Name (Utilities|Struct|BreakS_ItemInfos (.ItemInfos (Utilities|GetClassDefaults _output_get))))) (.Name (Utilities|Struct|BreakS_ItemInfos (.ItemInfos (Utilities|GetClassDefaults _output_get)))) _output_get_2 _output_get (Math|Float|Round (* (* (.Value (Utilities|Struct|BreakS_ItemInfos (.ItemInfos (Utilities|GetClassDefaults _output_get)))) _output_get_2) 1.11))))
    (Variables|Default|SetQuestInfo (Utilities|Struct|Makes_QuestInfo (Utilities|Text|FormatText "Collect {quantity}x {name}" _output_get_2 (.Name (Utilities|Struct|BreakS_ItemInfos (.ItemInfos (Utilities|GetClassDefaults _output_get))))) "NewEnumerator2" (Utilities|Text|FormatText "You are requested for {element}, find or get{quantity} of them  from your garden and deliver them." (.Name (Utilities|Struct|BreakS_ItemInfos (.ItemInfos (Utilities|GetClassDefaults _output_get)))) _output_get_2) (Utilities|Struct|Makes_QuestReward (Math|Float|Round (* (* (.Value (Utilities|Struct|BreakS_ItemInfos (.ItemInfos (Utilities|GetClassDefaults _output_get)))) _output_get_2) 1.11))) (Utilities|Array|MakeArray _structout)))
    (else
      (bind _output_get_3 (Variables|Default|SetPotion (Utilities|Array|Get(acopy) _allpotionitemclass (Math|Random|RandomInteger (Utilities|Array|Length _allpotionitemclass)))))
      (bind _output_get_4 (Variables|Default|SetDesiredPotions (Math|Random|RandomIntegerinRange 1 5)))
      (bind _structout_2 (Utilities|Struct|Setmembersins_GoalInfo (Utilities|Array|Get(acopy) (.SubGoals (Utilities|Struct|Breaks_QuestInfo (Variables|Default|GetQuestInfo)))) "NewEnumerator2" (.Name (Utilities|Struct|BreakS_ItemInfos (.ItemInfos (Utilities|GetClassDefaults _output_get_3)))) _output_get_4 _output_get_3 (Math|Float|Round (* (* (.Value (Utilities|Struct|BreakS_ItemInfos (.ItemInfos (Utilities|GetClassDefaults _output_get_3)))) _output_get_4) 1.5))))
      (Variables|Default|SetQuestInfo (Utilities|Struct|Makes_QuestInfo (Utilities|Text|FormatText "Delivery of {quantity}x {name}" _output_get_4 (.Name (Utilities|Struct|BreakS_ItemInfos (.ItemInfos (Utilities|GetClassDefaults _output_get_3))))) "NewEnumerator1" (Utilities|Text|FormatText "You are requested for {element}, make {quantity} of them and deliver them." (.Name (Utilities|Struct|BreakS_ItemInfos (.ItemInfos (Utilities|GetClassDefaults _output_get_3)))) _output_get_4) (Utilities|Struct|Makes_QuestReward (Math|Float|Round (* (* (.Value (Utilities|Struct|BreakS_ItemInfos (.ItemInfos (Utilities|GetClassDefaults _output_get_3)))) _output_get_4) 1.5))) (Utilities|Array|MakeArray _structout_2))))))

(fn ConstructionScript
  (|CallParentFunction))

(fn CreateClassfromGoalInfo
  (params (SubGoal :type S%20Goal%20Info%20Structure))
  (bind (_type _customgoal_ _goaltext _additionalname _amount _location _updatequestdescription_ _updateddescription _followingsubgoalindices _goalclass _goalid _useradius_ _radius _circlecolor _failmeansquestfail_ _completesquest_ _reward) (Utilities|Struct|Breaks_GoalInfo SubGoal))
  (Variables|Default|SetQuestInfo (Utilities|Struct|Makes_QuestInfo (Utilities|Text|FormatText "{Sarting} {quantity}x {name}" _amount _additionalname (Utilities|String|SelectString "Collect" "Delivery of" _customgoal_)) (Utilities|Select :Index _type :NewEnumerator0 "NewEnumerator0" :NewEnumerator1 "NewEnumerator2" :NewEnumerator2 "NewEnumerator1" :NewEnumerator3 "NewEnumerator0") (Utilities|Text|FormatText "You are requested for {element}, make {quantity} of them and deliver them." _additionalname _amount) (Utilities|Struct|Makes_QuestReward _reward) (Utilities|Array|MakeArray ""))))
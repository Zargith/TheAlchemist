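; Merchant inventory that stores items as class-and-amount slots and can be filled from an offer list.
; BeginPlay sizes the slot array and creates the main widget bound to this inventory.
; Adding merges into the first matching stack without a size cap, else takes an empty slot; removal checks the total, then drains matching slots.
; Item info comes from class defaults, so actors spawn only when an item is used.
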(event Custom|UseItemAtIndex
  (params (Index :type Integer))
  (bind _slots (Variables|Default|GetSlots))
  (bind _output (Utilities|Array|Get(acopy) _slots Index))
  (bind _itemclass (Utilities|Struct|BreakS_InventorySlot _output))
  (if (Utilities|IsValidClass _itemclass)
    (bind _returnvalue (Game|SpawnActorfromClass :Class _itemclass :CollisionHandlingOverride "AlwaysSpawn" :Inventory self :Index Index :Instigator 0))
    (Default|EventonUsed _returnvalue)))

(event EventBeginPlay
  (Utilities|Array|Resize (Variables|Default|GetSlots) (Variables|Default|GetAmoutOfSlots))
  (bind _returnvalue (UserInterface|CreateWidget "/Game/Systems/MainWidget.MainWidget_C" 0 self (Variables|Default|GetSlotsPerRow) 0.0 0))
  (bind _output_get (Variables|Default|SetMainWidget _returnvalue))
  (Variables|Default|SetInventoryWidget (Variables|/Game/Systems/MainWidget.MainWidget_C|GetInventoryWidget _output_get)))

(fn ConstructionScript)

(fn IsSlotEmpty?
  (params (Index :type Integer))
  (return (not (Utilities|IsValidClass (.itemClass (Utilities|Struct|BreakS_InventorySlot (Utilities|Array|Get(acopy) (Variables|Default|GetSlots) Index)))))))

(fn GetInfosatIndex
  (params (Index :type Integer))
  (bind _slots (Variables|Default|GetSlots))
  (bind _output (Utilities|Array|Get(acopy) _slots Index))
  (bind (_itemclass _amout) (Utilities|Struct|BreakS_InventorySlot _output))
  (if (Utilities|IsValidClass _itemclass)
    (return false (.ItemInfos (Utilities|GetClassDefaults _itemclass)) _amout)
    (else
      (return true "" 0))))

(fn SearchEmptySlot
  (bind (_array_element _array_index) (Utilities|Array|ForEachLoopwithBreak (Variables|Default|GetSlots) :!label _label)
    (:LoopBody
      (if (not (Utilities|IsValidClass (.itemClass (Utilities|Struct|BreakS_InventorySlot _array_element))))
        (LocalVariables|SetLocalBool true)
        (LocalVariables|SetLocalIndex _array_index)
        (goto _label Break)))
    (:Completed
      (return (LocalVariables|GetLocalBool) (LocalVariables|GetLocalIndex)))))

(fn SearchFreeStack
  (params (itemClass :type BP%20Master%20Item%20Class%20Reference))
  (bind (_array_element _array_index) (Utilities|Array|ForEachLoopwithBreak (Variables|Default|GetSlots) :!label _label)
    (:LoopBody
      (if (and (Utilities|IsValidClass (.itemClass (Utilities|Struct|BreakS_InventorySlot _array_element))) (== (.itemClass (Utilities|Struct|BreakS_InventorySlot _array_element)) itemClass))
        (LocalVariables|SetLocalBool true)
        (LocalVariables|SetLocalIndex _array_index)
        (goto _label Break)))
    (:Completed
      (return (LocalVariables|GetLocalBool) (LocalVariables|GetLocalIndex)))))

(fn AddItem
  (params (ItemClass :type BP%20Master%20Item%20Class%20Reference) (Amount :type Integer))
  (bind (_success_ _rest) (CallFunction|AddItem(internal) ItemClass Amount))
  (return _success_ _rest))

(fn AddItem(internal)
  (params (ItemClass :type BP%20Master%20Item%20Class%20Reference) (Amount :type Integer))
  (LocalVariables|SetLocalClass ItemClass)
  (LocalVariables|SetLocalAmount Amount)
  (bind (_success_ _index) (CallFunction|SearchFreeStack (LocalVariables|GetLocalClass)))
  (if _success_
    (bind _output_get (LocalVariables|SetFoundIndex _index))
    (Utilities|Array|SetArrayElem (Variables|Default|GetSlots) _output_get (Utilities|Struct|MakeS_InventorySlot (LocalVariables|GetLocalClass) (+ (.Amout (Utilities|Struct|BreakS_InventorySlot (Utilities|Array|Get(acopy) (Variables|Default|GetSlots) (LocalVariables|GetFoundIndex)))) (LocalVariables|GetLocalAmount))))
    (return true 0)
    (else
      (bind (_success__2 _index_2) (CallFunction|SearchEmptySlot))
      (if _success__2
        (LocalVariables|SetFoundIndex _index_2)
        (Utilities|Array|SetArrayElem (Variables|Default|GetSlots) (LocalVariables|GetFoundIndex) (Utilities|Struct|MakeS_InventorySlot (LocalVariables|GetLocalClass) (LocalVariables|GetLocalAmount)))
        (return true 0)
        (else
          (return false (LocalVariables|GetLocalAmount)))))))

(fn GetTotalAmountOfItem
  (params (Item :type BP%20Master%20Item%20Class%20Reference))
  (LocalVariables|SetLocalItem Item)
  (for (_array_element _array_index) (Variables|Default|GetSlots)
    (if (Utilities|IsValidClass (.itemClass (Utilities|Struct|BreakS_InventorySlot _array_element)))
      (if (== (.itemClass (Utilities|Struct|BreakS_InventorySlot _array_element)) (LocalVariables|GetLocalItem))
        (Utilities|Array|Add (LocalVariables|GetLocalIndexes) _array_index)
        (LocalVariables|SetLocalAmount (+ (LocalVariables|GetLocalAmount) (.Amout (Utilities|Struct|BreakS_InventorySlot _array_element)))))))
  (return (LocalVariables|GetLocalAmount) (LocalVariables|GetLocalIndexes)))

(fn RemoveItem
  (params (Item :type BP%20Master%20Item%20Class%20Reference) (Amount :type Integer))
  (bind (_totalamount _slotindexes) (CallFunction|GetTotalAmountOfItem Item))
  (if (>= _totalamount Amount)
    (bind _output_get (LocalVariables|SetLocalSlotIndexes _slotindexes))
    (LocalVariables|SetAmountToRemove Amount)
    (bind _array_element (Utilities|Array|ForEachLoopwithBreak _output_get :!label _label)
      (:LoopBody
        (if (< (CallFunction|GetAmountatIndex _array_element) (LocalVariables|GetAmountToRemove))
          (LocalVariables|SetAmountToRemove (- (LocalVariables|GetAmountToRemove) (CallFunction|GetAmountatIndex _array_element)))
          (CallFunction|RemoveItematIndex _array_element (CallFunction|GetAmountatIndex _array_element))
          (else
            (CallFunction|RemoveItematIndex _array_element (LocalVariables|GetAmountToRemove))
            (LocalVariables|SetAmountToRemove 0)
            (goto _label Break))))
      (:Completed
        (return true)))
    (else
      (return false))))

(fn GetAmountatIndex
  (params (Index :type Integer))
  (return (.Amout (Utilities|Struct|BreakS_InventorySlot (Utilities|Array|Get(acopy) (Variables|Default|GetSlots) Index)))))

(fn RemoveItematIndex
  (params (Index :type Integer) (Amount :type Integer))
  (bind _slots (Variables|Default|GetSlots))
  (bind _output_get (LocalVariables|SetLocalIndex Index))
  (bind _output_get_2 (LocalVariables|SetLocalAmount Amount))
  (if (and (not (CallFunction|IsSlotEmpty? _output_get)) (> _output_get_2 0))
    (if (>= (LocalVariables|GetLocalAmount) (CallFunction|GetAmountatIndex (LocalVariables|GetLocalIndex)))
      (Utilities|Array|SetArrayElem (Variables|Default|GetSlots) (LocalVariables|GetLocalIndex) (Utilities|Struct|MakeS_InventorySlot 0 0))
      (return true)
      (else
        (Utilities|Array|SetArrayElem _slots (LocalVariables|GetLocalIndex) (Utilities|Struct|MakeS_InventorySlot (.itemClass (Utilities|Struct|BreakS_InventorySlot (Utilities|Array|Get(acopy) _slots (LocalVariables|GetLocalIndex)))) (- (.Amout (Utilities|Struct|BreakS_InventorySlot (Utilities|Array|Get(acopy) _slots (LocalVariables|GetLocalIndex)))) (LocalVariables|GetLocalAmount))))
        (return true)))
    (else
      (return false))))

(fn FillInventory
  (params (Offer :type Array%20of%20S%20Merchant%20Slot%20Structures))
  (for _array_element Offer
    (CallFunction|AddItem (.ItemClass (Utilities|Struct|BreakS_MerchantSlot _array_element)) (.Quantity (Utilities|Struct|BreakS_MerchantSlot _array_element))))
  (return))
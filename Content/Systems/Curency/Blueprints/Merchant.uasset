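; Merchant actor in the currency system that players can approach, with empty hooks for interaction and shop closing.
; Its sphere overlap registers it as the player's NearByMerchant and shows MerchantText, then clears both when the player leaves.
; OnInteract, OnShopClosed and ComponentsToSave have no logic here.
; An IsNotStandingStill? helper branches on non-zero velocity but is not called by the event logic.
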(event OnComponentBeginOverlap(Sphere)
  (params (OverlappedComponent :type Primitive%20Component%20Object%20Reference) (OtherActor :type Actor%20Object%20Reference) (OtherComp :type Primitive%20Component%20Object%20Reference) (OtherBodyIndex :type Integer) (bFromSweep :type Boolean) (SweepResult :type Hit%20Result%20Structure%20%28by%20ref%29))
  (bind _asbp_player (Utilities|Casting|CastToBP_Player OtherActor))
  (Variables|/Game/Blueprints/BP_Player.BP_Player_C|SetNearByMerchant _asbp_player self)
  (Rendering|SetVisibility (Variables|Default|GetMerchantText) true false))

(event OnComponentEndOverlap(Sphere)
  (params (OverlappedComponent :type Primitive%20Component%20Object%20Reference) (OtherActor :type Actor%20Object%20Reference) (OtherComp :type Primitive%20Component%20Object%20Reference) (OtherBodyIndex :type Integer))
  (bind _asbp_player (Utilities|Casting|CastToBP_Player OtherActor))
  (Variables|/Game/Blueprints/BP_Player.BP_Player_C|SetNearByMerchant _asbp_player 0)
  (Rendering|SetVisibility (Variables|Default|GetMerchantText) false false))

(event Custom|OnInteract
  (params (PlayerRef :type BP%20Player%20Object%20Reference)))

(event Custom|OnShopClosed)

(fn ConstructionScript)

(fn ComponentstoSave
  (return 0))